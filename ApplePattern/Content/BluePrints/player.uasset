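; Player actor for an apple-catching game, moved sideways by the player and scoring when it hits an Apple.
; The Horizontal axis offsets it along world Y by Speed without delta-time scaling, then screen projection and deprojection clamp it between Cut and viewport width plus Cut.
; On a hit with an Apple, it sets that apple's IsOffScreen flag, increments Score and prints the total.
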(event Collision|EventActorBeginOverlap
  (params (OtherActor :type Actor%20Object%20Reference)))

(event Collision|EventHit
  (params (MyComp :type Primitive%20Component%20Object%20Reference) (Other :type Actor%20Object%20Reference) (OtherComp :type Primitive%20Component%20Object%20Reference) (bSelfMoved :type Boolean) (HitLocation :type Vector :default "0, 0, 0") (HitNormal :type Vector :default "0, 0, 0") (NormalImpulse :type Vector :default "0, 0, 0") (Hit :type Hit%20Result%20Structure%20%28by%20ref%29))
  (if (== (Utilities|GetClass Other) "/Game/BluePrints/Apple.Apple_C")
    (bind _asapple (Utilities|Casting|CastToApple Other))
    (Variables|/Game/BluePrints/Apple.Apple_C|SetIs%20Off%20Screen _asapple true)
    (bind _output_get (Variables|Default|SetScore (+ (Variables|Default|GetScore) 1)))
    (Development|PrintString (Utilities|String|ToString(Integer) _output_get))))

(event Input|AxisEvents|InputAxisHorizontal
  (params (AxisValue :type Float%20%28single-precision%29))
  (bind _returnvalue (Transformation|GetActorLocation))
  (bind _returnvalue_2 (Game|GetPlayerController 0))
  (bind _returnvalue_3 (Transformation|GetActorLocation))
  (bind _returnvalue_4 (Viewport|GetViewportSize))
  (bind _cut (Variables|Default|Getcut))
  (bind _screenposition (Class|GameplayStatics|ProjectWorldtoScreen _returnvalue_2 _returnvalue false))
  (bind _returnvalue_5 (+ (.x _returnvalue_4) _cut))
  (Transformation|AddActorWorldOffset (Math|Vector|MakeVector 0.0 (* AxisValue (Variables|Default|Getspeed)) 0.0))
  (Utilities|FlowControl|Sequence
    (:then_0
      (if (< (.x _screenposition) _cut)
        (Transformation|SetActorLocation (Math|Vector|MakeVector (.x _returnvalue_3) (.y (.WorldPosition (Class|GameplayStatics|DeprojectScreentoWorld _returnvalue_2 (Math|Vector2D|MakeVector2D _cut 0.0)))) (.z _returnvalue_3)) false false)))
    (:then_1
      (if (> (.x _screenposition) _returnvalue_5)
        (Transformation|SetActorLocation (Math|Vector|MakeVector (.x _returnvalue_3) (.y (.WorldPosition (Class|GameplayStatics|DeprojectScreentoWorld _returnvalue_2 (Math|Vector2D|MakeVector2D _returnvalue_5 0.0)))) (.z _returnvalue_3)) false false)))))

(fn ConstructionScript)