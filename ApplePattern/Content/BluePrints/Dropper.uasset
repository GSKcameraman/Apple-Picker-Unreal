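; Dropper is an actor that sweeps back and forth along the world Y axis, bouncing between the sides of the screen.
; BeginPlay sets the Cube's physics linear velocity from Velocity.
; Tick projects the actor location to screen space and negates Velocity whenever X reaches the Cut margin at either viewport edge.
; Actor overlaps only print an "Apple out!" message; nothing is spawned here.
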(event EventBeginPlay
  (Physics|SetPhysicsLinearVelocity (Variables|Default|GetCube) (Math|Vector|MakeVector 0.0 (Variables|Default|Getvelocity) 0.0) false "None"))

(event Collision|EventActorBeginOverlap
  (params (OtherActor :type Actor%20Object%20Reference))
  (Development|PrintString "Apple out!"))

(event EventTick
  (params (DeltaSeconds :type Float%20%28single-precision%29))
  (bind _returnvalue (Game|GetPlayerController 0))
  (bind _returnvalue_2 (Transformation|GetActorLocation))
  (bind _cut (Variables|Default|Getcut))
  (bind _screenposition (Class|GameplayStatics|ProjectWorldtoScreen _returnvalue _returnvalue_2 false))
  (if (or (<= (.x _screenposition) _cut) (>= (.x _screenposition) (- (.x (Viewport|GetViewportSize)) _cut)))
    (bind _output_get (Variables|Default|Setvelocity (* -1 (Variables|Default|Getvelocity))))
    (Physics|SetPhysicsLinearVelocity (Variables|Default|GetCube) (Math|Vector|MakeVector 0.0 _output_get 0.0) false "None")))

(fn ConstructionScript)