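; Apple actor that repeatedly falls from a dropper and recycles itself once it drops off the bottom of the screen.
; BeginPlay waits a random short delay, then MoveToDropper teleports it to the Dropper and zeroes its sphere's physics velocity.
; Tick projects its position to screen space; once below the viewport, it parks at DropPos, then returns to the Dropper after another random delay.
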(event EventBeginPlay
  (Utilities|FlowControl|Delay (Math|Random|RandomFloatinRange 0.5 2.0))
  (CallFunction|MovetoDropper))

(event Collision|EventActorBeginOverlap
  (params (OtherActor :type Actor%20Object%20Reference)))

(event EventTick
  (params (DeltaSeconds :type Float%20%28single-precision%29))
  (if (Variables|Default|GetIs%20Off%20Screen)
    (Transformation|SetActorLocation (Transformation|GetActorLocation (Variables|Default|GetDropPos)) false false)
    (Variables|Default|SetIs%20Off%20Screen false)
    (Utilities|FlowControl|Delay (Math|Random|RandomFloatinRange 0.5 2.0))
    (CallFunction|MovetoDropper)
    (elif (> (.y (.ScreenPosition (Class|GameplayStatics|ProjectWorldtoScreen (Game|GetPlayerController 0) (Transformation|GetActorLocation) false))) (+ (.y (Viewport|GetViewportSize)) 1e+01))
      (if (not (Variables|Default|GetIs%20Off%20Screen))
        (Variables|Default|SetIs%20Off%20Screen true)))))

(fn ConstructionScript)

(fn MovetoDropper
  (Transformation|SetActorLocation (Transformation|GetActorLocation (Variables|Default|GetDropper)) false true)
  (Physics|SetPhysicsLinearVelocity (Variables|Default|GetSphere) "0, 0, 0" false "None"))